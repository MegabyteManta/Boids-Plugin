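; BP_Boid is a boid actor that changes color when it heads for a collision.
; On BeginPlay it binds ChangeColor to the OnHeadedForCollision dispatcher and creates a dynamic instance of M_BoidColor on its static mesh.
; Each ChangeColor call sets that material's Color parameter to a random RGBA value, as a purely visual effect.
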(event Custom|ChangeColor
  ;[1 1 1] Fun colors when they head for a collision
  (Rendering|Material|SetVectorParameterValue (Variables|Default|GetDynamicMaterial) "Color" (Utilities|Struct|MakeLinearColor (Math|Random|RandomFloatinRange 0.0 1.0) (Math|Random|RandomFloatinRange 0.0 1.0) (Math|Random|RandomFloatinRange 0.0 1.0) (Math|Random|RandomFloatinRange 0.0 1.0)) :!class /Script/Engine.MaterialInstanceDynamic))

(event EventBeginPlay
  ;[1 1 1] Fun colors when they head for a collision
  (EventDispatchers|BindEventtoOnHeadedforCollision (delegate Custom|ChangeColor))
  (bind _returnvalue (Rendering|Material|CreateDynamicMaterialInstance (Variables|Default|GetStaticMesh) 0 "/Clavula/Materials/M_BoidColor.M_BoidColor" "None" :!class /Script/Engine.PrimitiveComponent))
  (Variables|Default|SetDynamicMaterial _returnvalue))

(fn ConstructionScript)